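; BP_Door is an interactable door that the player opens and closes with the E key while standing nearby.
; A Box trigger enables input and prints a prompt when a BP_Runner enters, then disables input and prints a leave message on exit.
; Pressing E alternates through a FlipFlop between playing and reversing a Timeline, whose track drives the static mesh's yaw to swing the door.
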(event `self.Box.OnComponentBeginOverlap`
  (params (OverlappedComponent :type "PrimitiveComponent Object Reference") (OtherActor :type "Actor Object Reference") (OtherComp :type "PrimitiveComponent Object Reference") (OtherBodyIndex :type Integer) (bFromSweep :type Boolean) (SweepResult :type "HitResult Structure (by ref)"))
  ;[1 1 1] 进入门的提示
  (cast `/Game/_Game/BP/Input/BP_Runner` OtherActor)
  (`self.EnableInput` (`GameplayStatics.GetPlayerController` 0))
  (`KismetSystemLibrary.PrintString` "开门输入 E"))

(event `self.Box.OnComponentEndOverlap`
  (params (OverlappedComponent :type "PrimitiveComponent Object Reference") (OtherActor :type "Actor Object Reference") (OtherComp :type "PrimitiveComponent Object Reference") (OtherBodyIndex :type Integer))
  ;[1 1 1] 进入门的提示
  (cast `/Game/_Game/BP/Input/BP_Runner` OtherActor)
  (`self.DisableInput` (`GameplayStatics.GetPlayerController` 0))
  (`KismetSystemLibrary.PrintString` "你已离开上帝之门"))

(event `Key|E`
  (params (Key :type "Key Structure"))
  ;[1 1 1] 按E 开关门
  (:`Pressed`
    (`/Engine/EditorBlueprintResources/StandardMacros.FlipFlop`
      (:`A`
        (bind (_direction `_新建轨道_0`) (`Timeline|时间轴` :!label _label)
          (:`Update`
            (`SceneComponent.K2_SetRelativeRotation` (`self.StaticMesh`) (`KismetMathLibrary.MakeRotator` 0.0 0.0 `_新建轨道_0`) false false))))
      (:`B`
        (goto _label :!via `ReverseFromEnd`)))))

(fn `UserConstructionScript`)