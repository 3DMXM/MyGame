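; BP_HitObgect is a moving obstacle actor that reacts when BP_Runner, the player, hits it.
; The first hit turns its mesh red and sets IsHit after a short delay; a later hit plays an explosion sound and particle, then destroys the actor.
; Tick moves it along a normalized Direction at Speed without sweeping, while a looping timer reverses that direction every TimeToChange seconds.
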(event `self.ReceiveHit`
  (params (MyComp :type "PrimitiveComponent Object Reference") (Other :type "Actor Object Reference") (OtherComp :type "PrimitiveComponent Object Reference") (bSelfMoved :type Boolean) (HitLocation :type "Vector Structure") (HitNormal :type "Vector Structure") (NormalImpulse :type "Vector Structure") (Hit :type "HitResult Structure (by ref)"))
  ;[1 1 1] 碰撞后的操作
  ;;[1 1 1] 判断是否是玩家
  (cast `/Game/_Game/BP/Input/BP_Runner` Other)
  (if (`self.IsHit`)
    ;;[1 1 1] 爆炸
    (`GameplayStatics.PlaySoundAtLocation` "/Game/StarterContent/Audio/Explosion01.Explosion01" HitLocation (struct) 1.0 1.0 0.0 null null null null)
    (`GameplayStatics.SpawnEmitterAttached` "/Game/StarterContent/Particles/P_Explosion.P_Explosion" null "None" HitLocation)
    (`self.K2_DestroyActor`)
    (else
      ;;[1 1 1] 进行变色
      (`PrimitiveComponent.SetMaterial` (`self.StaticMesh`) 0 "/Game/_Game/Mat/Mat_RedM.Mat_RedM")
      (`KismetSystemLibrary.Delay` 1.0)
      (set `self.IsHit` true))))

(event `self.ReceiveBeginPlay`
  ;[1 1 1] 定时器
  (`KismetSystemLibrary.K2_SetTimerDelegate` (delegate `ChangeDirection`) (`self.TimeToChange`) true))

(event `ChangeDirection`
  ;[1 1 1] 定时器
  (set `self.Direction` (* (`self.Direction`) -1)))

(event `self.ReceiveTick`
  (params (DeltaSeconds :type "Float (single-precision)"))
  ;[1 1 1] 定时器
  ;;[1 1 1] 移动
  (`self.K2_AddActorWorldOffset` (* (`KismetMathLibrary.Normal` (`self.Direction`)) (* (`self.Speed`) (`GameplayStatics.GetWorldDeltaSeconds`)))))

(fn `UserConstructionScript`)