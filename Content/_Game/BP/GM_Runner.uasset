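; GM_Runner is the runner game's mode Blueprint, handling coin-collection win logic and save/load.
; BeginPlay counts BP_Actor instances as the coin total; AddCoinCount increments BP_Runner's count or, on the last coin, calls ShowSucess to show WBP_Over with UI-only input.
; SaveGame and LoadGame transfer coin count and player location through BP_SaveGame.
; LoadGame's existence check uses an empty slot name, unlike the "SaveGame" slot it reads.
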(event `self.ReceiveBeginPlay`
  (bind _outactors (`GameplayStatics.GetAllActorsOfClass` "/Game/_Game/BP/BP_Actor.BP_Actor_C"))
  (set `self.Coins` (`KismetArrayLibrary.Array_Length` _outactors)))

(event `ShowSucess`
  (bind _returnvalue (`GameplayStatics.GetPlayerController` 0))
  ;[1 1 1] 显示通关提示
  (bind _returnvalue_2 (`|CreateWidget` "/Game/_Game/UI/WBP_Over.WBP_Over_C"))
  (`UserWidget.AddToViewport` _returnvalue_2 0)
  (`WidgetBlueprintLibrary.SetInputMode_UIOnlyEx` _returnvalue _returnvalue_2)
  (set `PlayerController.bShowMouseCursor` true _returnvalue)
  (`Controller.SetIgnoreMoveInput` _returnvalue false))

(event `SaveGame`
  ;[1 1 1] 保存游戏
  (bind _returnvalue (`GameplayStatics.CreateSaveGameObject` "/Game/_Game/BP/BP_SaveGame.BP_SaveGame_C"))
  (bind _asbp_runner (cast `/Game/_Game/BP/Input/BP_Runner` (`GameplayStatics.GetPlayerCharacter` 0)))
  (set `/Game/_Game/BP/BP_SaveGame.CoinCount` (`/Game/_Game/BP/Input/BP_Runner.CoinCount` _asbp_runner) _returnvalue)
  (set `/Game/_Game/BP/BP_SaveGame.Location` (`self.K2_GetActorLocation` _asbp_runner) _returnvalue)
  (`GameplayStatics.SaveGameToSlot` _returnvalue "SaveGame")
  (`KismetSystemLibrary.PrintString` "保存游戏"))

(event `LoadGame`
  (`GameplayStatics.DoesSaveGameExist` "")
  (if true
    (bind _returnvalue (`GameplayStatics.LoadGameFromSlot` "SaveGame"))
    (bind _asbp_save_game (cast `/Game/_Game/BP/BP_SaveGame` _returnvalue))
    (bind _asbp_runner (cast `/Game/_Game/BP/Input/BP_Runner` (`GameplayStatics.GetPlayerCharacter` 0)))
    (set `/Game/_Game/BP/Input/BP_Runner.CoinCount` (`/Game/_Game/BP/BP_SaveGame.CoinCount` _asbp_save_game) _asbp_runner)
    (`self.K2_SetActorLocation` _asbp_runner (`/Game/_Game/BP/BP_SaveGame.Location` _asbp_save_game) false false)
    (`KismetSystemLibrary.PrintString` "加载游戏")))

(fn `AddCoinCount`
  (params (Object :type "Object Object Reference"))
  (bind _asbp_runner (cast `/Game/_Game/BP/Input/BP_Runner` Object))
  (bind _coincount (`/Game/_Game/BP/Input/BP_Runner.CoinCount` _asbp_runner))
  (if (>= _coincount (- (`self.Coins`) 1))
    (`self.ShowSucess`)
    (else
      (`/Engine/EditorBlueprintResources/StandardMacros.IncrementInt` _coincount))))

(fn `UserConstructionScript`)