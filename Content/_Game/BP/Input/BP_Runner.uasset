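; BP_Runner is a player-controlled runner pawn with basic move and look controls through Enhanced Input.
; On BeginPlay it adds the IMC_Runner_Input mapping context to player 0's input subsystem.
; IAR_Move drives movement along right and forward vectors from the control rotation with pitch zeroed, so looking up or down does not tilt movement.
; IAR_Look feeds controller yaw and pitch, with the Y axis inverted.
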(event `self.ReceiveBeginPlay`
  ;[1 1 1] 输入
  (`EnhancedInputSubsystemInterface.AddMappingContext` (pcsubsystem `EnhancedInputLocalPlayerSubsystem` (`GameplayStatics.GetPlayerController` 0)) "/Game/_Game/BP/Input/IMC_Runner_Input.IMC_Runner_Input" 0 (struct)))

(event `EnhancedInput|/Game/_Game/BP/Input/Action/IAR_Move`
  (params (ActionValue :type "Vector2D Structure") (ElapsedSeconds :type "Float (double-precision)") (TriggeredSeconds :type "Float (double-precision)") (InputAction :type "InputAction Object Reference" :default "/Game/_Game/BP/Input/Action/IAR_Move.IAR_Move"))
  (bind (_returnvalue_roll _returnvalue_pitch _returnvalue_yaw) (`KismetMathLibrary.BreakRotator` (`self.GetControlRotation`)))
  ;[1 1 1] 输入
  (:`Triggered`
    (`self.AddMovementInput` (`KismetMathLibrary.GetRightVector` (`KismetMathLibrary.MakeRotator` _returnvalue_roll 0.0 _returnvalue_yaw)) ActionValue_X)
    (`self.AddMovementInput` (`KismetMathLibrary.GetForwardVector` (`KismetMathLibrary.MakeRotator` _returnvalue_roll 0.0 _returnvalue_yaw)) ActionValue_Y)))

(event `EnhancedInput|/Game/_Game/BP/Input/Action/IAR_Look`
  (params (ActionValue :type "Vector2D Structure") (ElapsedSeconds :type "Float (double-precision)") (TriggeredSeconds :type "Float (double-precision)") (InputAction :type "InputAction Object Reference" :default "/Game/_Game/BP/Input/Action/IAR_Look.IAR_Look"))
  ;[1 1 1] 输入
  (:`Triggered`
    (`self.AddControllerYawInput` ActionValue_X)
    (`self.AddControllerPitchInput` (* ActionValue_Y -1.0))))

(fn `UserConstructionScript`)